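; BP_EnemyShooter is an enemy actor that fires one telegraphed bullet at the player shortly after play begins.
; PrepareAttack locks the aim from FirePoint0 toward player 0 and spawns a BP_AttackWarning along that line, sized by WarningLength.
; After WarningDuration it spawns BP_EnemyBullet with the saved start and rotation, so the shot follows the warning, then destroys the warning.
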(event Custom|PrepareAttack
  (bind _output_get (Variables|Default|SetShotStart (Transformation|GetWorldLocation (Variables|Default|GetFirePoint_0))))
  (Variables|Default|SetShotRotation (Math|Rotator|FindLookatRotation _output_get (Transformation|GetActorLocation (Game|GetPlayerCharacter 0))))
  (bind _returnvalue (Game|SpawnActorfromClass "/Game/Personal/Yamada/BP/BP_AttackWarning.BP_AttackWarning_C" (Math|Transform|MakeTransform "0, 0, 0") "Undefined" "MultiplyWithRoot" 0 (Variables|Default|GetShotStart) (+ (* (Math|Vector|GetForwardVector (Variables|Default|GetShotRotation)) (Variables|Default|GetWarningLength)) (Variables|Default|GetShotStart)) 5.0 0))
  (Variables|Default|SetWarningActor _returnvalue)
  (Utilities|FlowControl|Delay (Variables|Default|GetWarningDuration))
  (Game|SpawnActorfromClass "/Game/Personal/Yamada/BP/BP_EnemyBullet.BP_EnemyBullet_C" (Math|Transform|MakeTransform (Variables|Default|GetShotStart) (Variables|Default|GetShotRotation)) "AlwaysSpawn" "MultiplyWithRoot" 0 0)
  (Actor|DestroyActor (Variables|Default|GetWarningActor)))

(event EventBeginPlay
  (Utilities|FlowControl|Delay 2.0)
  (CallFunction|PrepareAttack))

(event Collision|EventActorBeginOverlap
  (params (OtherActor :type Actor%20Object%20Reference)))

(event EventTick
  (params (DeltaSeconds :type Float%20%28single-precision%29)))

(fn ConstructionScript)