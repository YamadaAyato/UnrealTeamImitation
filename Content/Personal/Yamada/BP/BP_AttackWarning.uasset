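; BP_AttackWarning is an actor that shows an attack warning as a straight line between a start point and an end point.
; UpdateWarning moves the actor to the midpoint, rotates it toward the end point, and scales WarningMesh by the distance and LineWidth.
; It runs from both the Construction Script and BeginPlay, so the line is laid out at construction and again when play begins.
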(event EventBeginPlay
  (CallFunction|UpdateWarning))

(event Collision|EventActorBeginOverlap
  (params (OtherActor :type Actor%20Object%20Reference)))

(event EventTick
  (params (DeltaSeconds :type Float%20%28single-precision%29)))

(fn ConstructionScript
  (CallFunction|UpdateWarning))

(fn UpdateWarning
  (bind _linewidth (Variables|Default|GetLineWidth))
  (bind _returnvalue (/ _linewidth 1e+02))
  (Transformation|SetActorLocation (* (+ (Variables|Default|GetStartPoint) (Variables|Default|GetEndPoint)) (Math|Conversions|ToVector(Float) 0.5)) false false)
  (Transformation|SetActorRotation (Math|Rotator|FindLookatRotation (Variables|Default|GetStartPoint) (Variables|Default|GetEndPoint)))
  (Transformation|SetRelativeScale3D (Variables|Default|GetWarningMesh) (Math|Vector|MakeVector (/ (Math|Vector|Distance(Vector) (Variables|Default|GetStartPoint) (Variables|Default|GetEndPoint)) 1e+02) _returnvalue _returnvalue)))