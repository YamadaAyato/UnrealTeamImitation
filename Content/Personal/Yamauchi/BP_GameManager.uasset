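; Game manager that runs one play session from start to result screen and on to the next stage.
; BeginPlay shows the in-game panel and starts BPTimer and BPDistance on it, with a fixed delay triggering the clear event.
; Clearing stores time and distance in a BP_Result appended to BP_BGameInstance's result array.
; It then shows the result panel and, after another delay, fades to MoveStageName.
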(event Custom|ClearEvent
  (bind _bptimer (Variables|Default|GetBPTimer))
  (bind _bpdistance (Variables|Default|GetBPDistance))
  (Class|BPIIClear|Clear(Message) _bptimer)
  (Class|BPIIClear|Clear(Message) _bpdistance)
  (bind _returnvalue (Game|ConstructObjectfromClass (Game|GetGameInstance) "/Game/Personal/Yamauchi/BP_Result.BP_Result_C" (Variables|/Game/Personal/Yamauchi/BP_Timer.BP_Timer_C|GetTime _bptimer) (Variables|/Game/Personal/Yamauchi/BP_Distance.BP_Distance_C|GetDistance _bpdistance)))
  (bind _asbp_bgame_instance (Utilities|Casting|CastToBP_BGameInstance (Game|GetGameInstance)))
  (Default|AddResultArray _asbp_bgame_instance _returnvalue)
  (CallFunction|ResultEvent))

(event Custom|GameStart
  (Default|EventTimerStart (Variables|Default|GetBPTimer) (stale EventBeginPlay _returnvalue))
  (Default|MeasureDistance (Variables|Default|GetBPDistance) (stale EventBeginPlay _returnvalue))
  (Utilities|FlowControl|Delay 4.0)
  (CallFunction|ClearEvent))

(event Custom|ResultEvent
  (bind _returnvalue (UserInterface|CreateWidget "/Game/Personal/Yamauchi/WBP_ResultPanel.WBP_ResultPanel_C"))
  (UserInterface|Viewport|AddtoViewport _returnvalue 0)
  (Default|ResultEvent _returnvalue (Variables|/Game/Personal/Yamauchi/BP_Distance.BP_Distance_C|GetDistance (Variables|Default|GetBPDistance)) (Variables|/Game/Personal/Yamauchi/BP_Timer.BP_Timer_C|GetTime (Variables|Default|GetBPTimer)))
  (Utilities|FlowControl|Delay 5.0)
  (CallFunction|FadeStageMove (Variables|Default|GetMoveStageName)))

(event EventBeginPlay
  (bind _returnvalue (UserInterface|CreateWidget "/Game/Personal/Yamauchi/WBP_IngamePanel.WBP_IngamePanel_C"))
  (UserInterface|Viewport|AddtoViewport _returnvalue 0)
  (Default|CallGameStartEvent)
  (CallFunction|GameStart))

(fn ConstructionScript)