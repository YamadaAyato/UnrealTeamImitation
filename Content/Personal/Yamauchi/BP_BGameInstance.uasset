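; Game instance Blueprint that holds a ranking of results, each compared by distance and timer, and tracks the most recently added one.
; AddResultArray appends a result and stores it as the current one.
; ReadResult runs a two-pass swap sort, ascending by distance and then timer for equal distances, then trims the stored array to the requested rank count.
; It returns the list and the current result's index within it.
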(fn AddResultArray
  (params (Result :type BP%20Result%20Object%20Reference))
  (Utilities|Array|Add (Variables|Default|GetResultArray) Result)
  (Variables|Default|SetCurrentResult Result))

(fn ReadResult
  (params (Rank :type Integer))
  (bind _resultarray (Variables|Default|GetResultArray))
  (Variables|Default|SetRank Rank)
  (if (> (Utilities|Array|Length (Variables|Default|GetResultArray)) 1)
    (CallFunction|MySort "None")
    (CallFunction|MySort "Then")
    (CallFunction|MyTake))
  (return _resultarray (Utilities|Array|FindItem _resultarray (Variables|Default|GetCurrentResult))))

(fn MySort
  (params (SortKind :type Name))
  (bind _resultarray (Variables|Default|GetResultArray))
  (bind _returnvalue (Utilities|Array|Length _resultarray))
  (bind _returnvalue_2 (- _returnvalue 1))
  (for _index (range 0 _returnvalue_2)
    (for _index_2 (range _index _returnvalue_2)
      (if (== SortKind "Then")
        (if (== (Variables|/Game/Personal/Yamauchi/BP_Result.BP_Result_C|GetDistance (Utilities|Array|Get(acopy) _resultarray _index)) (Variables|/Game/Personal/Yamauchi/BP_Result.BP_Result_C|GetDistance (Utilities|Array|Get(acopy) _resultarray _index_2)))
          (if (> (Variables|/Game/Personal/Yamauchi/BP_Result.BP_Result_C|GetTimer (Utilities|Array|Get(acopy) _resultarray _index)) (Variables|/Game/Personal/Yamauchi/BP_Result.BP_Result_C|GetTimer (Utilities|Array|Get(acopy) _resultarray _index_2)))
            (Utilities|Array|Swap _resultarray _index _index_2)))
        (elif (> (Variables|/Game/Personal/Yamauchi/BP_Result.BP_Result_C|GetDistance (Utilities|Array|Get(acopy) _resultarray _index)) (Variables|/Game/Personal/Yamauchi/BP_Result.BP_Result_C|GetDistance (Utilities|Array|Get(acopy) _resultarray _index_2)))
          (Utilities|Array|Swap _resultarray _index _index_2))))))

(fn MyTake
  (bind _resultarray (Variables|Default|GetResultArray))
  (bind _rank (Variables|Default|GetRank))
  (if (> (Utilities|Array|Length (Variables|Default|GetResultArray)) _rank)
    (bind _output_get (LocalVariables|SetRArray _resultarray))
    (Utilities|Array|Clear _resultarray)
    (for _index (range 0 (- _rank 1))
      (Utilities|Array|Add _resultarray (Utilities|Array|Get(acopy) _output_get _index)))))